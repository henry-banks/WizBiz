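; MenuController is a player controller that owns and switches the game's menu and end screen widgets.
; BeginPlay sets UI-only input focused on MainMenu, with no mouse lock.
; Separate init functions create and store either the main menu with stats, info and options screens, or the end screen, showing only the main or end widget.
; SwitchUI removes all widgets and adds the requested one to the viewport.
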(event `self.ReceiveBeginPlay`
  (`WidgetBlueprintLibrary.SetInputMode_UIOnlyEx` self (`self.MainMenu`)))

(fn `Init UI End Screen`
  (bind _returnvalue (`|CreateWidget` "/Game/Blueprint/UMG/EndScreen.EndScreen_C" self))
  (bind _output_get (set `self.EndScreen` _returnvalue))
  (`UserWidget.AddToViewport` _output_get 0))

(fn `Init UI Main Menu`
  (bind _returnvalue (`|CreateWidget` "/Game/Blueprint/UMG/MainMenu.MainMenu_C" self))
  (bind _output_get (set `self.MainMenu` _returnvalue))
  (`UserWidget.AddToViewport` _output_get 0)
  (bind _returnvalue_2 (`|CreateWidget` "/Game/Blueprint/UMG/StatsScreen.StatsScreen_C" self))
  (set `self.StatsScreen` _returnvalue_2)
  (bind _returnvalue_3 (`|CreateWidget` "/Game/Blueprint/UMG/InfoScreen.InfoScreen_C" self))
  (set `self.infoScreen` _returnvalue_3)
  (bind _returnvalue_4 (`|CreateWidget` "/Game/Blueprint/UMG/OptionsScreen.OptionsScreen_C" self))
  (set `self.OptionsScreen` _returnvalue_4))

(fn `switchUI`
  (params (`new UI` :type "UserWidget Object Reference"))
  (`WidgetLayoutLibrary.RemoveAllWidgets`)
  (`UserWidget.AddToViewport` `new UI` 0))

(fn `UserConstructionScript`)