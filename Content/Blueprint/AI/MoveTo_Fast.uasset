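; Behavior tree task that moves an AI-controlled enemy pawn to its follow target.
; On execute, it casts the owner to EnemyController and caches it if not already valid.
; It then runs AIMoveTo toward the blackboard actor with a small acceptance radius and finishes the task as success or failure from the move result.
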(event `self.ReceiveExecute`
  (params (OwnerActor :type "Actor Object Reference"))
  (`/Engine/EditorBlueprintResources/StandardMacros.IsValid` (`self.ControllerRef`)
    (:`Is Valid`
      _)
    (:`Is Not Valid`
      (bind _asenemy_controller (cast `/Game/Blueprint/AI/EnemyController` OwnerActor))
      (set `self.ControllerRef` _asenemy_controller)))
  (`|AIMoveTo` (`Controller.K2_GetPawn` (`self.ControllerRef`)) (0.0 0.0 0.0) (`BTFunctionLibrary.GetBlackboardValueAsActor` (`self.FollowTarget`)) 50.0
    (:`OnSuccess`
      (`self.FinishExecute` true))
    (:`OnFail`
      (`self.FinishExecute` false))))