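; Enemy character that kills itself on contact, either dying to damage or exploding on the player.
; On BeginPlay it reads WizInstance and, in hard mode, doubles its damage and sets a faster walk speed.
; Capsule overlap with a "Damage" tag counts a kill; a "Character" tag spawns an explosion and damages the player.
; An EventDie event also removes it, updating the game instance's kill and live-enemy counters.
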(event `self.ReceiveBeginPlay`
  (bind _aswiz_instance (cast `/Game/Blueprint/WizInstance` (`GameplayStatics.GetGameInstance`))
    (:`then`
      (bind _output_get (set `self.gameInstance` _aswiz_instance))
      (if (`/Game/Blueprint/WizInstance.isHardMode` _output_get)
        (set `self.damage` (* (`self.damage`) 2))
        (if (`/Game/Blueprint/WizInstance.isHardMode` (`self.gameInstance`))
          (set `CharacterMovementComponent.MaxWalkSpeed` 600.0 (`self.CharacterMovement`)))))
    (:`CastFailed`
      (`KismetSystemLibrary.PrintString` "Enemy could not cast to instance"))))

(event `self.CapsuleComponent.OnComponentBeginOverlap`
  (params (OverlappedComponent :type "PrimitiveComponent Object Reference") (OtherActor :type "Actor Object Reference") (OtherComp :type "PrimitiveComponent Object Reference") (OtherBodyIndex :type Integer) (bFromSweep :type Boolean) (SweepResult :type "HitResult Structure (by ref)"))
  (bind _componenttags (`ActorComponent.ComponentTags` OtherComp))
  (bind _gameinstance (`self.gameInstance`))
  (if (`KismetArrayLibrary.Array_Contains` _componenttags "Damage")
    (`GameplayStatics.PlaySoundAtLocation` "/Game/FirstPerson/Audio/FirstPersonTemplateWeaponFire02.FirstPersonTemplateWeaponFire02" (`self.K2_GetActorLocation`))
    (`/Engine/EditorBlueprintResources/StandardMacros.IncrementInt` (`/Game/Blueprint/WizInstance.killedEnemies` _gameinstance)
      (:`  `
        (`/Engine/EditorBlueprintResources/StandardMacros.DecrementInt` (`/Game/Blueprint/WizInstance.currentEnemies` _gameinstance) :!label _label
          (:`  `
            (`self.K2_DestroyActor`)))))
    (elif (`KismetArrayLibrary.Array_Contains` _componenttags "Character")
      (`|SpawnActorFromClass` "/Game/StarterContent/Blueprints/Blueprint_Effect_Explosion.Blueprint_Effect_Explosion_C" (`self.GetTransform`) "Undefined" "OverrideRootScale" null self)
      (bind _asfirst_person_character (cast `/Game/FirstPersonCPP/Blueprints/FirstPersonCharacter` (`GameplayStatics.GetPlayerPawn` 0))
        (:`then`
          (`/Game/FirstPersonCPP/Blueprints/FirstPersonCharacter.Event Damage` _asfirst_person_character (`self.damage`))
          (goto _label))
        (:`CastFailed`
          (`KismetSystemLibrary.PrintString` "COULD NOT CAST TO PLAYER"))))))

(event `EventDie`
  (params (isKilled :type Boolean))
  (if isKilled
    (`GameplayStatics.PlaySoundAtLocation` "/Game/FirstPerson/Audio/FirstPersonTemplateWeaponFire02.FirstPersonTemplateWeaponFire02" (`self.K2_GetActorLocation`))
    (`/Engine/EditorBlueprintResources/StandardMacros.IncrementInt` (`/Game/Blueprint/WizInstance.killedEnemies` (`self.gameInstance`))
      (:`  `
        _)))
  (`/Engine/EditorBlueprintResources/StandardMacros.DecrementInt` (`/Game/Blueprint/WizInstance.currentEnemies` (`self.gameInstance`))
    (:`  `
      (`self.K2_DestroyActor`))))

(fn `UserConstructionScript`)