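; AgroCheck is an enemy AI behavior tree node, likely a service, that keeps the blackboard aimed at the player.
; On tick it caches the owning EnemyController, then checks player controller 0's death flag as a WizBizController.
; While the player lives, it writes that controller, not the pawn, to FollowTarget and its location to TargetLocation, with no range check.
; A dead or missing player clears only FollowTarget.
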(event `self.ReceiveTick`
  (params (OwnerActor :type "Actor Object Reference") (DeltaSeconds :type "Float (single-precision)"))
  (bind _returnvalue (`GameplayStatics.GetPlayerController` 0))
  (`/Engine/EditorBlueprintResources/StandardMacros.IsValid` (`self.ControllerRef`)
    (:`Is Valid`
      (`/Engine/EditorBlueprintResources/StandardMacros.IsValid` _returnvalue :!label _label
        (:`Is Valid`
          (bind _aswiz_biz_controller (cast `/Game/Blueprint/WizBizController` _returnvalue))
          (if (`/Game/Blueprint/WizBizController.isDead` _aswiz_biz_controller)
            (`BTFunctionLibrary.SetBlackboardValueAsObject` (`self.FollowTarget`) :!label _label_2)
            (else
              (`BTFunctionLibrary.SetBlackboardValueAsObject` (`self.FollowTarget`) _returnvalue)
              (`BTFunctionLibrary.SetBlackboardValueAsVector` (`self.TargetLocation`) (`Actor.K2_GetActorLocation` _returnvalue)))))
        (:`Is Not Valid`
          (`KismetSystemLibrary.PrintString` "AgroCheck: no player controller!")
          (goto _label_2))))
    (:`Is Not Valid`
      (bind _asenemy_controller (cast `/Game/Blueprint/AI/EnemyController` OwnerActor)
        (:`then`
          (set `self.ControllerRef` _asenemy_controller)
          (goto _label))
        (:`CastFailed`
          (`KismetSystemLibrary.PrintString` "Agro Check: Cast to EnemyController failed"))))))