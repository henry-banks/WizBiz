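; Pickup spawner actor that keeps one pickup of a configurable class at its spawn point, replacing it after it is gone.
; BeginPlay spawns the first pickup, passing spin settings to it, and starts a looping respawn timer that is immediately paused.
; Tick polls the pickup's validity, unpausing the timer while the pickup is missing and pausing it again once a new one exists.
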(event `self.ReceiveBeginPlay`
  (`self.Event Spawn`)
  (bind _returnvalue (`KismetSystemLibrary.K2_SetTimerDelegate` (delegate `Event Spawn`) (`self.spawnInterval`) true))
  (bind _output_get (set `self.spawnTimer` _returnvalue))
  (`KismetSystemLibrary.K2_PauseTimerHandle` _output_get))

(event `Event Spawn`
  (bind _returnvalue (`|SpawnActorFromClass` (`self.pickupToSpawn`) (`KismetMathLibrary.MakeTransform` (`SceneComponent.K2_GetComponentLocation` (`self.SpawnPoint`))) "Undefined" "OverrideRootScale" self (`self.isSpin`) (`self.spinAmount`)))
  (set `self.pickup` _returnvalue))

(event `self.ReceiveTick`
  (params (DeltaSeconds :type "Float (single-precision)"))
  (bind _returnvalue (`KismetSystemLibrary.K2_IsTimerPausedHandle` (`self.spawnTimer`)))
  (`/Engine/EditorBlueprintResources/StandardMacros.IsValid` (`self.pickup`)
    (:`Is Valid`
      (if (not _returnvalue)
        (`KismetSystemLibrary.K2_PauseTimerHandle` (`self.spawnTimer`))))
    (:`Is Not Valid`
      (if _returnvalue
        (`KismetSystemLibrary.K2_UnPauseTimerHandle` (`self.spawnTimer`))))))

(fn `UserConstructionScript`)