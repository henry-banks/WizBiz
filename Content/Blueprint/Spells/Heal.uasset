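; Heal spell Blueprint that restores health to its owning character, extending a parent spell class.
; On BeginPlay it attaches with location and rotation snapped to the target.
; Each SpellEffect call runs the parent logic, then the owner's mana check, setting IsActive false on failure.
; On success it adds HealAmount only if the result stays within MaxHealth, so a heal that would overshoot is skipped rather than clamped.
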(event `self.ReceiveBeginPlay`
  (`parent.ReceiveBeginPlay`)
  (`self.K2_AttachToComponent` (`self.parent`) "None" "SnapToTarget" "SnapToTarget" "KeepRelative"))

(event `self.ReceiveTick`
  (params (DeltaSeconds :type "Float (single-precision)"))
  (`parent.ReceiveTick` DeltaSeconds))

(event `self.SpellEffect`
  (bind _ownerchar (`self.ownerChar`))
  (bind _returnvalue (+ (`/Game/FirstPersonCPP/Blueprints/FirstPersonCharacter.currentHealth` _ownerchar) (`self.healAmount`)))
  (`parent.SpellEffect`)
  (bind _issuccess (`/Game/FirstPersonCPP/Blueprints/FirstPersonCharacter.ManaCheck` (`self.ownerChar`) (`self.data`)))
  (if _issuccess
    (if (<= _returnvalue (`/Game/FirstPersonCPP/Blueprints/FirstPersonCharacter.maxHealth` _ownerchar))
      (set `/Game/FirstPersonCPP/Blueprints/FirstPersonCharacter.currentHealth` _returnvalue (`self.ownerChar`)))
    (else
      (set `self.isActive` false))))

(fn `UserConstructionScript`)