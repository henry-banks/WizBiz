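; DeathCircle is a spell actor that arms after a delay and removes itself when its lifetime runs out.
; It starts with its Cylinder hidden and its Capsule collision disabled.
; Tick counts down two timers: BoomTimer triggers a one-shot that shows the Cylinder, enables collision and activates the Earrape component, while Lifetime destroys the actor.
; No overlap or damage logic is implemented in this graph.
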(event `self.ReceiveBeginPlay`
  (`SceneComponent.SetVisibility` (`self.Cylinder`) false false)
  (`PrimitiveComponent.SetCollisionEnabled` (`self.Capsule`) "NoCollision"))

(event `self.ReceiveTick`
  (params (DeltaSeconds :type "Float (single-precision)"))
  (set `self.lifetime` (- (`self.lifetime`) DeltaSeconds))
  (set `self.boomTimer` (- (`self.boomTimer`) DeltaSeconds))
  (if (and (<= (`self.boomTimer`) 0.0) (not (`self.stopTimer`)))
    (`SceneComponent.SetVisibility` (`self.Cylinder`) true false)
    (`PrimitiveComponent.SetCollisionEnabled` (`self.Capsule`) "QueryAndPhysics")
    (`ActorComponent.Activate` (`self.earrape`) false)
    (set `self.stopTimer` true))
  (if (<= (`self.lifetime`) 0.0)
    (`self.K2_DestroyActor`)))

(fn `UserConstructionScript`)