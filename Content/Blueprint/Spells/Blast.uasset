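; Blast spell actor that acts as a short-lived explosion area, scaled uniformly by Radius in the construction script.
; On BeginPlay it spawns an explosion effect at its transform, slightly scaled down, and starts two one-shot timers.
; The DamageLifetime timer destroys the Capsule to stop damage, and the Lifetime timer destroys the actor.
; The graph itself contains no damage-dealing logic.
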(event `self.ReceiveBeginPlay`
  (`KismetSystemLibrary.K2_SetTimerDelegate` (delegate `stopDamage`) (`self.damageLifetime`))
  (`KismetSystemLibrary.K2_SetTimerDelegate` (delegate `d`) (`self.lifetime`))
  (`|SpawnActorFromClass` "/Game/StarterContent/Blueprints/Blueprint_Effect_Explosion.Blueprint_Effect_Explosion_C" (`KismetMathLibrary.MakeTransform` (.location (`self.GetTransform`)) (.rotation (`self.GetTransform`)) (* (.scale (`self.GetTransform`)) (0.8 0.8 0.8))) "Undefined" "OverrideRootScale"))

(event `stopDamage`
  (`ActorComponent.K2_DestroyComponent` (`self.Capsule`)))

(event `d`
  (`self.K2_DestroyActor`))

(fn `UserConstructionScript`
  (bind _radius (`self.radius`))
  (`self.SetActorScale3D` (`KismetMathLibrary.MakeVector` _radius _radius _radius)))