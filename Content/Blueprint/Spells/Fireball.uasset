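; Fireball spell projectile that explodes on hitting or overlapping any actor other than a FirstPersonCharacter.
; Impact destroys the mesh, spawns an explosion effect, stops movement and swaps the projectile collision for the initially disabled Damage collision.
; The construction script scales Damage by Radius, and a timer destroys the actor after ExplosionTimer.
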(event `self.ReceiveBeginPlay`
  (`PrimitiveComponent.SetCollisionEnabled` (`self.damage`) "NoCollision"))

(event `self.CollisionComp.OnComponentHit`
  (params (HitComponent :type "PrimitiveComponent Object Reference") (OtherActor :type "Actor Object Reference") (OtherComp :type "PrimitiveComponent Object Reference") (NormalImpulse :type "Vector Structure") (Hit :type "HitResult Structure (by ref)"))
  (cast `/Game/FirstPersonCPP/Blueprints/FirstPersonCharacter` OtherActor
    (:`CastFailed`
      (`ActorComponent.K2_DestroyComponent` (`self.Mesh`) :!label _label)
      (`|SpawnActorFromClass` "/Game/StarterContent/Blueprints/Blueprint_Effect_Explosion.Blueprint_Effect_Explosion_C" (`self.GetTransform`) "Undefined" "OverrideRootScale")
      (`PrimitiveComponent.SetCollisionEnabled` (`self.damage`) "QueryAndPhysics")
      (`PrimitiveComponent.SetCollisionEnabled` (`self.CollisionComp`) "NoCollision")
      (`MovementComponent.StopMovementImmediately` (`self.ProjectileMovement`))
      (`KismetSystemLibrary.K2_SetTimerDelegate` (delegate `die`) (`self.explosionTimer`)))))

(event `self.CollisionComp.OnComponentBeginOverlap`
  (params (OverlappedComponent :type "PrimitiveComponent Object Reference") (OtherActor :type "Actor Object Reference") (OtherComp :type "PrimitiveComponent Object Reference") (OtherBodyIndex :type Integer) (bFromSweep :type Boolean) (SweepResult :type "HitResult Structure (by ref)"))
  (cast `/Game/FirstPersonCPP/Blueprints/FirstPersonCharacter` OtherActor
    (:`CastFailed`
      (goto _label))))

(event `die`
  (`self.K2_DestroyActor`))

(fn `UserConstructionScript`
  (bind _radius (`self.radius`))
  (`SceneComponent.SetWorldScale3D` (`self.damage`) (`KismetMathLibrary.MakeVector` _radius _radius _radius)))