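; Spawn point actor that periodically spawns AI enemies at its own location while the enemy population is below a cap.
; Tick counts down an interval timer, then spawns the enemy class with its behavior tree and resets the timer.
; The WizInstance game instance, cached on BeginPlay, holds the cap and the current and total enemy counters, which each spawn increments.
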(event `self.ReceiveBeginPlay`
  (bind _aswiz_instance (cast `/Game/Blueprint/WizInstance` (`GameplayStatics.GetGameInstance`))
    (:`then`
      (set `self.gameInstance` _aswiz_instance))
    (:`CastFailed`
      _))
  (set `self.spawnTimer` (`self.SpawnInterval`)))

(event `self.ReceiveTick`
  (params (DeltaSeconds :type "Float (single-precision)"))
  (bind _gameinstance (`self.gameInstance`))
  (bind _spawntimer (`self.spawnTimer`))
  (bind _gameinstance_2 (`self.gameInstance`))
  (set `self.spawnTimer` (- _spawntimer DeltaSeconds))
  (if (and (<= _spawntimer 0.0) (< (`/Game/Blueprint/WizInstance.currentEnemies` _gameinstance) (`/Game/Blueprint/WizInstance.maxEnemies` _gameinstance)))
    (`AIBlueprintHelperLibrary.SpawnAIFromClass` "/Game/Blueprint/AI/enemyCharacter.enemyCharacter_C" "/Game/Blueprint/AI/EnemyBT.EnemyBT" (`self.K2_GetActorLocation`))
    (`/Engine/EditorBlueprintResources/StandardMacros.IncrementInt` (`/Game/Blueprint/WizInstance.currentEnemies` _gameinstance_2)
      (:`  `
        (`/Engine/EditorBlueprintResources/StandardMacros.IncrementInt` (`/Game/Blueprint/WizInstance.totalEnemies` _gameinstance_2)
          (:`  `
            (set `self.spawnTimer` (`self.SpawnInterval`))))))))

(fn `UserConstructionScript`)