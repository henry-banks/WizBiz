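; FocusSpell is a spell actor owned by the FirstPersonCharacter, with an empty SpellEffect function as the place for its effect.
; On BeginPlay it starts a looping timer that calls SpellEffect every TickInterval, then caches the owning character, fires SpellEffect once immediately and caches the WizInstance game instance.
; Tick destroys the actor once IsActive is false.
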(event `self.ReceiveBeginPlay`
  (bind _returnvalue (`KismetSystemLibrary.K2_SetTimer` null "SpellEffect" (`self.tickInterval`) true))
  (set `self.tickTimer` _returnvalue)
  (bind _asfirst_person_character (cast `/Game/FirstPersonCPP/Blueprints/FirstPersonCharacter` (`self.GetOwner`))
    (:`then`
      (set `self.ownerChar` _asfirst_person_character)
      (`self.SpellEffect`)
      (bind _aswiz_instance (cast `/Game/Blueprint/WizInstance` (`GameplayStatics.GetGameInstance`))
        (:`then`
          (set `self.instance` _aswiz_instance))
        (:`CastFailed`
          (`KismetSystemLibrary.PrintString` "Focus Spell failed cast to instance"))))
    (:`CastFailed`
      (`KismetSystemLibrary.PrintString` "Focus Spell failed cast to character"))))

(event `self.ReceiveTick`
  (params (DeltaSeconds :type "Float (single-precision)"))
  (if (not (`self.isActive`))
    (`self.K2_DestroyActor`)))

(fn `SpellEffect`)

(fn `UserConstructionScript`)