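; Base pickup actor that the first-person character collects by overlapping its sphere.
; On overlap it stores the character reference, calls the empty Effect and OnDeath hooks, increments the pickup count on the WizInstance game instance, then destroys itself.
; An optional yaw spin on the static mesh runs each tick at a configurable speed, scaled by delta time.
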(event `self.ReceiveBeginPlay`
  (bind _aswiz_instance (cast `/Game/Blueprint/WizInstance` (`GameplayStatics.GetGameInstance`)))
  (set `self.instance` _aswiz_instance))

(event `self.ReceiveTick`
  (params (DeltaSeconds :type "Float (single-precision)"))
  (if (`self.isSpin`)
    (`SceneComponent.K2_AddLocalRotation` (`self.StaticMesh`) (`KismetMathLibrary.MakeRotator` 0.0 0.0 (* DeltaSeconds (`self.spinAmount`))) false false)))

(event `self.Sphere.OnComponentBeginOverlap`
  (params (OverlappedComponent :type "PrimitiveComponent Object Reference") (OtherActor :type "Actor Object Reference") (OtherComp :type "PrimitiveComponent Object Reference") (OtherBodyIndex :type Integer) (bFromSweep :type Boolean) (SweepResult :type "HitResult Structure (by ref)"))
  (if (== (`GameplayStatics.GetObjectClass` OtherActor) "/Game/FirstPersonCPP/Blueprints/FirstPersonCharacter.FirstPersonCharacter_C")
    (bind _asfirst_person_character (cast `/Game/FirstPersonCPP/Blueprints/FirstPersonCharacter` OtherActor))
    (set `self.characterRef` _asfirst_person_character)
    (`self.Effect`)
    (`self.onDeath`)
    (`/Engine/EditorBlueprintResources/StandardMacros.IncrementInt` (`/Game/Blueprint/WizInstance.pickups` (`self.instance`))
      (:`  `
        (`self.K2_DestroyActor`)))))

(fn `Effect`)

(fn `onDeath`)

(fn `UserConstructionScript`)